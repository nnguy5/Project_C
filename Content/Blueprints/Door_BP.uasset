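; Door Blueprint meant to swing open when a key-carrying third-person character overlaps its Box trigger.
; The overlap checks the character's HasKey, then casts to Key_BP with no object connected, so execution stops there.
; Past that cast, Doorid is compared to a fixed 1, ignoring the key's ID, to play the OpenDoor yaw timeline.
; Missing or wrong keys are meant to print on-screen messages.
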(event `self.Box.OnComponentBeginOverlap`
  (params (OverlappedComponent :type "PrimitiveComponent Object Reference") (OtherActor :type "Actor Object Reference") (OtherComp :type "PrimitiveComponent Object Reference") (OtherBodyIndex :type Integer) (bFromSweep :type Boolean) (SweepResult :type "HitResult Structure (by ref)"))
  (bind _asbp_third_person_character (cast `/Game/ThirdPerson/Blueprints/BP_ThirdPersonCharacter` OtherActor))
  (if (`/Game/ThirdPerson/Blueprints/BP_ThirdPersonCharacter.HasKey` _asbp_third_person_character)
    (cast `/Game/Blueprints/Key_BP` _)
    (`/Game/Blueprints/Key_BP.getkeyID`)
    (if (== (`self.doorid`) 1)
      (bind (_direction _rotate) (`Timeline|OpenDoor`)
        (:`Update`
          (`SceneComponent.K2_SetRelativeRotation` (`self.Door`) (`KismetMathLibrary.MakeRotator` 0.0 0.0 _rotate) false false)))
      (else
        (`KismetSystemLibrary.PrintString` "Wrong Keu" true true (struct :`R` 1.0 :`G` 0.089796 :`B` 0.145538 :`A` 1.0))))
    (else
      (`KismetSystemLibrary.PrintString` "You need a key" true false))))

(fn `UserConstructionScript`)